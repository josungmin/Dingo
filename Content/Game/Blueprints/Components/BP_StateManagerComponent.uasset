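; BP_StateManagerComponent is a component that tracks its owner's current state and current character action as two separate values.
; Each setter ignores unchanged values, otherwise firing an end dispatcher for the old value and a begin dispatcher for the new one.
; Getters and list-based membership checks expose both values, and ResetState returns the state to a default enum entry.
; It holds no transition rules and runs no BeginPlay or Tick logic.
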(fn `Get Current Action`
  (returns (`Return Value` :type "/Game/Game/Blueprints/Enums/E_CharacterAction Enum"))
  (return (`self.Current Character Action`)))

(fn `Get Current State`
  (returns (`Current State` :type "/Game/Game/Blueprints/Enums/E_CharacterState Enum"))
  (return (`self.Current State`)))

(fn `IsCurrentAction`
  (params (ActionToCheck :type "Array of /Game/Game/Blueprints/Enums/E_CharacterAction Enum"))
  (returns (`Return Value` :type Boolean))
  (return (`KismetArrayLibrary.Array_Contains` ActionToCheck (`self.Current Character Action`))))

(fn `IsCurrentState`
  (params (`States to Chaeck` :type "Array of /Game/Game/Blueprints/Enums/E_CharacterState Enum"))
  (returns (`Return Value` :type Boolean))
  (return (`KismetArrayLibrary.Array_Contains` `States to Chaeck` (`self.Current State`))))

(fn `Reset State`
  (`self.Set State` "NewEnumerator0"))

(fn `Set Current Action`
  (params (`New Character Action` :type "/Game/Game/Blueprints/Enums/E_CharacterAction Enum" :default "NewEnumerator0"))
  (if (`|EnumInequality` `New Character Action` (`self.Current Character Action`))
    (`self.OnCharacterActionEnd` (`self.Current Character Action`))
    (bind _output_get (set `self.Current Character Action` (`local.New Character Action`)))
    (`self.OnCharacterActionBegin` _output_get)))

(fn `Set State`
  (params (`New State` :type "/Game/Game/Blueprints/Enums/E_CharacterState Enum" :default "NewEnumerator0"))
  (if (`|EnumInequality` `New State` (`self.Current State`))
    (`self.OnStateEnd` (`self.Current State`))
    (bind _output_get (set `self.Current State` (`local.New State`)))
    (`self.OnStateBegin` _output_get)))