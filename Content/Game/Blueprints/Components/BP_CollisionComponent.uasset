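; BP_CollisionComponent is a reusable component that detects hits along an assigned mesh while collision is enabled.
; Each Tick it runs a multi-sphere object trace between the mesh's start and end sockets, skipping an editable ignore list.
; New actors are recorded and broadcast once through OnHit; enabling collision clears that record, so each activation can hit them again.
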(event `Set Collision Mesh`
  (params (MeshComponent :type "PrimitiveComponent Object Reference"))
  (set `self.CollisionMeshComponent` MeshComponent))

(event `Enable Collision`
  (`self.Clear Hit Actors`)
  (set `self.bIsCollisionEnabled` true))

(event `Collision Trace`
  (bind _collisionmeshcomponent (`self.CollisionMeshComponent`))
  (bind _outhits (`KismetSystemLibrary.SphereTraceMultiForObjects` (`SceneComponent.GetSocketLocation` _collisionmeshcomponent (`self.Start Socket Name`)) (`SceneComponent.GetSocketLocation` _collisionmeshcomponent (`self.End Socket Name`)) (`self.Trace Radius`) (`self.Collision Object Types`) false (`self.Actors to Ignore`) (`self.Draw Debug Type`)))
  (for _array_element _outhits
    (bind _output_get (set `self.Last Hit` _array_element))
    (bind (_bblockinghit _binitialoverlap _time _distance _location _impactpoint _normal _impactnormal _physmat _hitactor) (`GameplayStatics.BreakHitResult` _output_get))
    (if (not (`KismetArrayLibrary.Array_Contains` (`self.AlreadyHitActors`) _hitactor))
      (bind _output_get_2 (set `self.Hit Actor` _hitactor))
      (`KismetArrayLibrary.Array_Add` (`self.AlreadyHitActors`) _output_get_2)
      (`self.OnHit` (`self.Last Hit`)))))

(event `Disable Collision`
  (set `self.bIsCollisionEnabled` false))

(event `Clear Hit Actors`
  (`KismetArrayLibrary.Array_Clear` (`self.AlreadyHitActors`)))

(event `self.ReceiveTick`
  (params (DeltaSeconds :type "Float (single-precision)"))
  (if (`self.bIsCollisionEnabled`)
    (`self.Collision Trace`)))

(fn `AddActorToIgnore`
  (params (InActor :type "Actor Object Reference (by ref)"))
  (`KismetArrayLibrary.Array_AddUnique` (`self.Actors to Ignore`) InActor))

(fn `GetActorToIgnore`
  (returns (`Return Value` :type "Array of Actor Object Reference"))
  (return (`self.Actors to Ignore`)))

(fn `GetAlreadyHitActors`
  (returns (`Return Value` :type "Array of Actor Object Reference"))
  (return (`self.AlreadyHitActors`)))

(fn `GetCollisionMeshComponent`
  (returns (`Return Value` :type "PrimitiveComponent Object Reference"))
  (return (`self.CollisionMeshComponent`)))

(fn `GetIsCollisionEnabled`
  (returns (`Return Value` :type Boolean))
  (return (`self.bIsCollisionEnabled`)))

(fn `GetLastHit`
  (returns (`Last Hit` :type "HitResult Structure"))
  (return (`self.Last Hit`)))

(fn `RemoveActorToIgnore`
  (params (InActor :type "Actor Object Reference (by ref)"))
  (`KismetArrayLibrary.Array_RemoveItem` (`self.Actors to Ignore`) InActor))