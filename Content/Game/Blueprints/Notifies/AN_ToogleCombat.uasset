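; AN_ToogleCombat is an animation notify that switches a character's combat mode on or off during an animation.
; On trigger it gets the owner's BP_CombatComponent and, if the main weapon is valid, attaches it to its hand socket or attach socket depending on EnableCombat.
; It then passes the same flag to SetCombatEnable on the component, returning false when no valid weapon exists.
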(fn `Received_Notify`
  (params (MeshComp :type "SkeletalMeshComponent Object Reference") (Animation :type "AnimSequenceBase Object Reference") (EventReference :type "AnimNotifyEventReference Structure (by ref)"))
  (returns (ReturnValue :type Boolean))
  (bind _returnvalue (`Actor.GetComponentByClass` (`ActorComponent.GetOwner` MeshComp) "/Game/Game/Blueprints/Components/BP_CombatComponent.BP_CombatComponent_C"))
  (bind _return_value (`/Game/Game/Blueprints/Components/BP_CombatComponent.GetMainWeapon` _returnvalue))
  (`/Engine/EditorBlueprintResources/StandardMacros.IsValid` _return_value
    (:`Is Valid`
      (`/Game/Game/Blueprints/Weapons/BP_BaseEquipable.Attach Actor` _return_value (select `bool` (`self.bEnableCombat`) :`false` (`/Game/Game/Blueprints/Weapons/BP_BaseEquipable.Attach Socket Name` _return_value) :`true` (`/Game/Game/Blueprints/Weapons/BP_BaseWeapon.Hand Socket Name` _return_value)))
      (`/Game/Game/Blueprints/Components/BP_CombatComponent.SetCombatEnable` _returnvalue (`self.bEnableCombat`))
      (return true))
    (:`Is Not Valid`
      (return false))))