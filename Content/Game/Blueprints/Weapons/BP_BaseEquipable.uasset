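; Base Blueprint for equipable items, likely weapons, that tracks equipped state and attaches to the owning character.
; OnEquipped sets the flag and calls AttachActor, which casts the owner to Character and snaps to AttachSocketName on its mesh.
; OnUnequipped only clears the flag, without detaching.
; GetItemMesh returns the static mesh component when it has a valid mesh, otherwise the skeletal one, as their shared Primitive Component type.
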(fn `Attach Actor`
  (params (SocketName :type Name))
  (bind _ascharacter (cast `Character` (`self.GetOwner`)))
  (`self.K2_AttachToComponent` (`Character.Mesh` _ascharacter) SocketName "SnapToTarget" "SnapToTarget" "SnapToTarget"))

(fn `GetIsEquipped`
  (returns (`Return Value` :type Boolean))
  (return (`self.bIsEquipeed`)))

(fn `GetItemMesh`
  (returns (`Return Value` :type "PrimitiveComponent Object Reference"))
  (`/Engine/EditorBlueprintResources/StandardMacros.IsValid` (`StaticMeshComponent.StaticMesh` (`self.ItemStaticMesh`))
    (:`Is Valid`
      (return (`self.ItemStaticMesh`)) ; 반환 자료형이 Primitive Component인 이유는 Static Mesh Component와 Skeletal Mesh Component의 Base Calss이기 때문이다
    )
    (:`Is Not Valid`
      (return (`self.ItemSkeletalMesh`)))))

(fn `OnEquipped`
  (set `self.bIsEquipeed` true)
  (`self.Attach Actor` (`self.Attach Socket Name`)))

(fn `OnUnequipped`
  (if (`self.bIsEquipeed`)
    (set `self.bIsEquipeed` false)))

(fn `SetIsEquipped`
  (params (`Input Value` :type Boolean))
  (set `self.bIsEquipeed` `Input Value`))

(fn `UserConstructionScript`)