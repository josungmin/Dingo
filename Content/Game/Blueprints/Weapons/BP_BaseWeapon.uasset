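; BP_BaseWeapon is a base melee weapon item that deals damage and supplies the montages for combat actions.
; On equip it attaches to the hand or stow socket by combat state, registers with the owner's BP_CombatComponent and sends its combat type to the AnimInstance.
; Its collision component traces the item mesh, ignoring the owner, and applies point damage to actors that can receive it.
; It can also switch the mesh to physics simulation.
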(event `self.BP_CollisionComponent.OnHit`
  (params (`Hit Result` :type "HitResult Structure"))
  (bind (_bblockinghit _binitialoverlap _time _distance _location _impactpoint _normal _impactnormal _physmat _hitactor) (`GameplayStatics.BreakHitResult` `Hit Result`))
  (bind _return_value (message `/Game/Game/Blueprints/Interfaces/BPI_Combat.CanRecieveDamage` _hitactor))
  (if _return_value
    (`GameplayStatics.ApplyPointDamage` _hitactor (`self.Damage`) (`self.GetActorForwardVector` (`self.GetOwner`)) `Hit Result` (`self.GetInstigatorController`) self)))

(event `Simulate Weapon Physics`
  (`PrimitiveComponent.SetCollisionProfileName` (`self.GetItemMesh`) "PhysicsActor" true)
  (`PrimitiveComponent.SetSimulatePhysics` (`self.GetItemMesh`) true))

(fn `Get Action Montages`
  (params (`Character Action` :type "/Game/Game/Blueprints/Enums/E_CharacterAction Enum" :default "NewEnumerator0"))
  (returns (`Return Value` :type "Array of AnimMontage Object Reference"))
  (return (select `/Game/Game/Blueprints/Enums/E_CharacterAction` `Character Action` :`NewEnumerator1` (`self.Light Attack Montages`) :`NewEnumerator2` (`self.Heavy Attack Montages`) :`NewEnumerator3` (`self.Charge Attack Montages`) :`NewEnumerator4` (`self.Falling Attack Montages`) :`NewEnumerator5` (`self.Dodge Montages`) :`NewEnumerator6` (`|MakeArray` (`self.Equip Montage`)) :`NewEnumerator7` (`|MakeArray` (`self.Unequip Montage`)))))

(fn `OnEquipped`
  (`parent.OnEquipped`)
  (set `self.CombatComponent` (`self.GetComponentByClass` (`self.GetOwner`) "/Game/Game/Blueprints/Components/BP_CombatComponent.BP_CombatComponent_C"))
  (`self.Attach Actor` (select `bool` (`/Game/Game/Blueprints/Components/BP_CombatComponent.GetCombatEnable` (`self.CombatComponent`)) :`false` (`self.Attach Socket Name`) :`true` (`self.Hand Socket Name`)))
  (`/Game/Game/Blueprints/Components/BP_CombatComponent.SetMainWeapon` (`self.CombatComponent`) self)
  (message `/Game/Game/Blueprints/Interfaces/BPI_CombatType.Update Combat Type` (`SkeletalMeshComponent.GetAnimInstance` (`Character.Mesh` (cast `Character` (`self.GetOwner`) :!pure true))) (`self.Combat Type`))
  (`/Game/Game/Blueprints/Components/BP_CollisionComponent.Set Collision Mesh` (`self.BP_CollisionComponent`) (`self.GetItemMesh`))
  (`/Game/Game/Blueprints/Components/BP_CollisionComponent.AddActorToIgnore` (`self.BP_CollisionComponent`) (`self.GetOwner`)))

(fn `UserConstructionScript`
  (`parent.UserConstructionScript`))